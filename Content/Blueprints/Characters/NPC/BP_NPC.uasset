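; BP_NPC is an NPC that faces the player and shows or hides a speech-bubble widget by proximity.
; Each tick it compares X position with the player and flips its render component 180 degrees to match.
; Box overlap begin and end by the player both call the same visibility toggle on WBP_NPCBubble.
; BeginPlay detaches the box and widget, keeping world transforms, so the flip leaves them unaffected.
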(event `self.ReceiveBeginPlay`
  (`SceneComponent.K2_DetachFromComponent` (`self.Box`) "KeepWorld" "KeepWorld" "KeepWorld" true)
  (`SceneComponent.K2_DetachFromComponent` (`self.Widget`) "KeepWorld" "KeepWorld" "KeepWorld" true))

(event `self.ReceiveTick`
  (params (DeltaSeconds :type "Float (single-precision)"))
  (bind _returnvalue_x (`KismetMathLibrary.BreakVector` (`self.K2_GetActorLocation`)))
  (bind _rendercomponent (`self.RenderComponent`))
  (bind _returnvalue_x_2 (`KismetMathLibrary.BreakVector` (`self.K2_GetActorLocation` (`GameplayStatics.GetPlayerCharacter` 0))))
  (if (>= _returnvalue_x _returnvalue_x_2)
    (`SceneComponent.K2_SetWorldRotation` _rendercomponent (struct :`Yaw` 180.0) false false)
    (else
      (`SceneComponent.K2_SetWorldRotation` :`self` _rendercomponent))))

(event `self.Box.OnComponentBeginOverlap`
  (params (OverlappedComponent :type "PrimitiveComponent Object Reference") (OtherActor :type "Actor Object Reference") (OtherComp :type "PrimitiveComponent Object Reference") (OtherBodyIndex :type Integer) (bFromSweep :type Boolean) (SweepResult :type "HitResult Structure (by ref)"))
  (cast `/Game/Blueprints/Characters/Player/BP_PlayerCharacter` OtherActor :!label _label)
  (bind _aswbp_npcbubble (cast `/Game/Blueprints/UI/HUD/WBP_NPCBubble` (`WidgetComponent.GetWidget` (`self.Widget`))))
  (`/Game/Blueprints/UI/HUD/WBP_NPCBubble.ChangeVisibility` _aswbp_npcbubble))

(event `self.Box.OnComponentEndOverlap`
  (params (OverlappedComponent :type "PrimitiveComponent Object Reference") (OtherActor :type "Actor Object Reference") (OtherComp :type "PrimitiveComponent Object Reference") (OtherBodyIndex :type Integer))
  (goto _label))

(fn `UserConstructionScript`)