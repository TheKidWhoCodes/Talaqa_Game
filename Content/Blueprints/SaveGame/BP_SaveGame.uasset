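; BP_SaveGame is a save game data container for player progression and level results.
; It stores player level, XP, XP to the next level, level completion, per-level stars and percentages, and a user document.
; SetValues writes all fields at once, while GetValues returns all of them except the user document.
; Neither function performs disk saving or loading.
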(fn `GetValues`
  (returns (PlayerLevel :type Integer) (PlayerXP :type Integer) (StarsPerLevel :type "Array of Integer") (XPToNextLevel :type Integer) (LevelCompleted :type "Array of Boolean") (PercentagePerLevel :type "Array of Float (double-precision)"))
  (return (`self.PlayerLevel`) (`self.PlayerXP`) (`self.StarsPerLevel`) (`self.XPToNextLevel`) (`self.LevelCompleted`) (`self.PercentagePerLevel`)))

(fn `SetValues`
  (params (PlayerLevel :type Integer) (PlayerXP :type Integer) (StarsPerLevel :type "Array of Integer") (XPToNextLevel :type Integer) (LevelCompleted :type "Array of Boolean") (UserDocument :type String) (PercentagePerLevel :type "Array of Float (double-precision)"))
  (set `self.PlayerLevel` PlayerLevel)
  (set `self.PlayerXP` PlayerXP)
  (set `self.StarsPerLevel` StarsPerLevel)
  (set `self.XPToNextLevel` XPToNextLevel)
  (set `self.LevelCompleted` LevelCompleted)
  (set `self.UserDocument` UserDocument)
  (set `self.PercentagePerLevel` PercentagePerLevel))