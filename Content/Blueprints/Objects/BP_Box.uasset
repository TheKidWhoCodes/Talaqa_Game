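; BP_Box is a box actor that is either a physics object or a static one, chosen by the Moveable flag.
; The construction script enables physics and removes the Box and CollisionBox components when Moveable, otherwise it disables physics.
; Overlapping Box starts the player character's speech and locks its movement, and actor end overlap reverses both.
; Hard impacts play a landing sound, and IsHit destroys the actor after a short delay.
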(event `self.ReceiveHit`
  (params (MyComp :type "PrimitiveComponent Object Reference") (Other :type "Actor Object Reference") (OtherComp :type "PrimitiveComponent Object Reference") (bSelfMoved :type Boolean) (HitLocation :type "Vector Structure") (HitNormal :type "Vector Structure") (NormalImpulse :type "Vector Structure") (Hit :type "HitResult Structure (by ref)"))
  (if (> (`KismetMathLibrary.VSize` NormalImpulse) 20000.0)
    (`GameplayStatics.PlaySound2D` "/Game/Audio/Land.Land" 1.0 1.0 0.0 null null)))

(event `IsHit`
  (`KismetSystemLibrary.Delay` 2.0)
  (`self.K2_DestroyActor`))

(event `self.Box.OnComponentBeginOverlap`
  (params (OverlappedComponent :type "PrimitiveComponent Object Reference") (OtherActor :type "Actor Object Reference") (OtherComp :type "PrimitiveComponent Object Reference") (OtherBodyIndex :type Integer) (bFromSweep :type Boolean) (SweepResult :type "HitResult Structure (by ref)"))
  (bind _asbp_player_character (cast `/Game/Blueprints/Characters/Player/BP_PlayerCharacter` OtherActor))
  (`/Game/Blueprints/Characters/Player/BP_PlayerCharacter.BeginSpeech` _asbp_player_character)
  (`/Game/Blueprints/Characters/Player/BP_PlayerCharacter.LockMovement` _asbp_player_character))

(event `self.ReceiveActorEndOverlap`
  (params (OtherActor :type "Actor Object Reference"))
  (bind _asbp_player_character (cast `/Game/Blueprints/Characters/Player/BP_PlayerCharacter` OtherActor))
  (`/Game/Blueprints/Characters/Player/BP_PlayerCharacter.EndSpeech` _asbp_player_character)
  (`/Game/Blueprints/Characters/Player/BP_PlayerCharacter.UnlockMovement` _asbp_player_character))

(fn `UserConstructionScript`
  (if (`self.bMoveable`)
    (`ActorComponent.K2_DestroyComponent` (`self.Box`))
    (`ActorComponent.K2_DestroyComponent` (`self.CollisionBox`))
    (`PrimitiveComponent.SetSimulatePhysics` (`self.RenderComponent`) true)
    (else
      (`PrimitiveComponent.SetSimulatePhysics` (`self.RenderComponent`) false))))