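; Player character for a 2D side-scrolling knight game where the player attacks boxes by speaking sentences aloud.
; Enhanced Input drives movement, jump and pause, while flipbook playback handles run/idle animation and frame-timed footsteps.
; BeginSpeech streams captured microphone audio into an Arabic speech recognizer; the HUD checks recognized words, triggering an attack on overlapping boxes or a retry.
; It also tracks health, showing the loss menu at zero, and exposes movement locking.
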(event `self.ReceiveTick`
  (params (DeltaSeconds :type "Float (single-precision)"))
  (bind _charactermovement (`self.CharacterMovement`))
  (bind _velocity_x (`KismetMathLibrary.BreakVector` (`MovementComponent.Velocity` _charactermovement)))
  (`self.UpdateAnimation`)
  (if (and (and (!= _velocity_x 0.0) (`NavMovementComponent.IsMovingOnGround` _charactermovement)) (select `int` (`PaperFlipbookComponent.GetPlaybackPositionInFrames` (`self.Sprite`)) :`0` false :`1` true :`2` false :`3` false :`4` true :`5` false))
    (`GameplayStatics.PlaySound2D` "/Game/Audio/FootStep.FootStep" 1.0 1.0 0.0 null null)))

(event `self.ReceiveBeginPlay`
  (`self.EnableInput` null)
  (bind _asplayer_controller (cast `PlayerController` (`self.GetController`)))
  (`WidgetBlueprintLibrary.SetInputMode_GameOnly` _asplayer_controller)
  (`EnhancedInputSubsystemInterface.AddMappingContext` (pcsubsystem `EnhancedInputLocalPlayerSubsystem` _asplayer_controller) "/Game/Blueprints/Input/IMC_Player.IMC_Player" 0 (struct))
  (bind _returnvalue (`|CreateWidget` "/Game/Blueprints/UI/HUD/WBP_HUD.WBP_HUD_C"))
  (bind _output_get (set `self.HUDWidget` _returnvalue))
  (`UserWidget.AddToViewport` _output_get 0)
  (`SceneComponent.K2_DetachFromComponent` (`self.Widget`) "KeepWorld" "KeepWorld" "KeepWorld" true))

(event `EnhancedInput|/Game/Blueprints/Input/IA_Move`
  (params (ActionValue :type "Float (double-precision)") (ElapsedSeconds :type "Float (double-precision)") (TriggeredSeconds :type "Float (double-precision)") (InputAction :type "InputAction Object Reference" :default "/Game/Blueprints/Input/IA_Move.IA_Move"))
  (bind _returnvalue (`GameplayStatics.GetPlayerController` 0))
  (:`Triggered`
    (if (`self.CanMove`)
      (if (> ActionValue 0.0)
        (`Controller.SetControlRotation` _returnvalue (`KismetMathLibrary.MakeRotator` 0.0))
        (else
          (`Controller.SetControlRotation` _returnvalue (`KismetMathLibrary.MakeRotator` 0.0 0.0 180.0))))
      (`self.AddMovementInput` (1.0 0.0 0.0) ActionValue)
      (`self.BeginWidgetAnimation`))))

(event `EnhancedInput|/Game/Blueprints/Input/IA_Jump`
  (params (ActionValue :type Boolean) (ElapsedSeconds :type "Float (double-precision)") (TriggeredSeconds :type "Float (double-precision)") (InputAction :type "InputAction Object Reference" :default "/Game/Blueprints/Input/IA_Jump.IA_Jump"))
  (:`Triggered`
    (if (`self.CanMove`)
      (if (not (`NavMovementComponent.IsFalling` (`self.CharacterMovement`)))
        (`self.Jump`)
        (`GameplayStatics.PlaySound2D` "/Game/Audio/CartoonJump.CartoonJump" 1.0 1.0 0.0 null null)
        (`self.BeginWidgetAnimation`)
        (`PaperFlipbookComponent.SetPlaybackPositionInFrames` (`self.Sprite`) 1 false)
        (`PaperFlipbookComponent.SetPlayRate` (`self.Sprite`) 0.0)))))

(event `self.OnLanded`
  (params (Hit :type "HitResult Structure (by ref)"))
  (`GameplayStatics.PlaySound2D` "/Game/Audio/Land.Land" 1.0 1.0 0.0 null null)
  (`PaperFlipbookComponent.SetPlayRate` (`self.Sprite`) 1.0))

(event `EnhancedInput|/Game/Blueprints/Input/IA_Pause`
  (params (ActionValue :type Boolean) (ElapsedSeconds :type "Float (double-precision)") (TriggeredSeconds :type "Float (double-precision)") (InputAction :type "InputAction Object Reference" :default "/Game/Blueprints/Input/IA_Pause.IA_Pause"))
  (:`Triggered`
    (if (not (`GameplayStatics.IsGamePaused`))
      (bind _returnvalue (`|CreateWidget` "/Game/Blueprints/UI/HUD/WBP_PauseMenu.WBP_PauseMenu_C"))
      (`UserWidget.AddToViewport` _returnvalue 0))))

(event `BeginWidgetAnimation`
  (`/Engine/EditorBlueprintResources/StandardMacros.DoOnce` false
    (:`Completed`
      (bind _aswbp_controls_widget (cast `/Game/Blueprints/UI/HUD/WBP_ControlsWidget` (`WidgetComponent.GetWidget` (`self.Widget`))))
      (`/Game/Blueprints/UI/HUD/WBP_ControlsWidget.BeginFade` _aswbp_controls_widget))))

(event `BeginSpeech`
  (bind _hudwidget (`self.HUDWidget`)
    (:`then`
      (`/Game/Blueprints/UI/HUD/WBP_HUD.ShowSentence` _hudwidget)
      (`KismetSystemLibrary.Delay` 1.0)
      (set `self.State` "NewEnumerator1")
      (bind _returnvalue (`SpeechRecognizer.CreateSpeechRecognizer`))
      (bind _output_get (set `self.SpeechRecognizer` _returnvalue))
      (add `SpeechRecognizer.OnRecognitionFinished` _output_get (delegate `OnRecognitionFinished_Event`))
      (add `SpeechRecognizer.OnRecognitionError` (`self.SpeechRecognizer`) (delegate `OnRecognitionError_Event`))
      (add `SpeechRecognizer.OnRecognizedTextSegment` (`self.SpeechRecognizer`) (delegate `OnRecognizedTextSegment_Event`))
      (`SpeechRecognizer.SetStreamingDefaults` (`self.SpeechRecognizer`))
      ;[1 1 1] Language Settings
      (`SpeechRecognizer.SetLanguage` (`self.SpeechRecognizer`) "Ar")
      (`SpeechRecognizer.StartSpeechRecognition` (`self.SpeechRecognizer`) (delegate `OnStartSpeechRecognition_Event`))
      (`KismetSystemLibrary.PrintString` "CAPTURE STARTED" true true (struct :`R` 1.0 :`A` 1.0)))
    (:`else`)))

(event `OnRecognitionError_Event`
  (params (ShortErrorMessage :type String) (LongErrorMessage :type String))
  (`KismetSystemLibrary.PrintString` LongErrorMessage true true (struct :`R` 1.0 :`A` 1.0) 15.0))

(event `OnStartSpeechRecognition_Event`
  (params (bSucceeded :type Boolean))
  ;[1 1 1] Start of capture
  (bind _returnvalue (`CapturableSoundWave.CreateCapturableSoundWave`))
  (bind _output_get (set `self.CapturableSoundWave` _returnvalue))
  (add `ImportedSoundWave.OnPopulateAudioData` _output_get (delegate `OnPopulateAudioData_Event`))
  (`CapturableSoundWave.StartCapture` (`self.CapturableSoundWave`) 1))

(event `OnRecognitionFinished_Event`
  ;[1 1 1] On Recognition Finished (Recording stops)
  (if (not (`CapturableSoundWave.IsCapturing` (`self.CapturableSoundWave`)))
    (`SpeechRecognizer.StopSpeechRecognition` (`self.SpeechRecognizer`))
    (set `self.SpeechRecognizer` null)
    (`KismetSystemLibrary.PrintString` "CAPTURE ENDED" true true (struct :`R` 1.0 :`A` 1.0))))

(event `OnPopulateAudioData_Event`
  (params (PopulatedAudioData :type "Array of Float (single-precision) (by ref)"))
  (bind _capturablesoundwave (`self.CapturableSoundWave`))
  (`SpeechRecognizer.ProcessAudioData` (`self.SpeechRecognizer`) PopulatedAudioData (`KismetMathLibrary.Conv_IntToDouble` (`ImportedSoundWave.GetSampleRate` _capturablesoundwave)) (`ImportedSoundWave.GetNumOfChannels` _capturablesoundwave) false) ; If this causes issues convert speech rec. node to validated
)

(event `EndSpeech`
  ;[1 1 1] End of capture
  (`CapturableSoundWave.StopCapture` (`self.CapturableSoundWave`))
  (bind _speechrecognizer (`self.SpeechRecognizer`)
    (:`then`
      (`SpeechRecognizer.ForceProcessPendingAudioData` _speechrecognizer) ; If this causes issues convert speech rec. node to validated
    )
    (:`else`)))

(event `OnRecognizedTextSegment_Event`
  (params (RecognizedWords :type String))
  ;[1 1 1] On Recognition (User input is recognized)
  (bind _shouldendspeech (`/Game/Blueprints/UI/HUD/WBP_HUD.CheckUserInput` (`self.HUDWidget`) RecognizedWords))
  (if _shouldendspeech
    (`GameplayStatics.PlaySound2D` "/Game/Audio/CorrectInput.CorrectInput" 1.0 1.0 0.0 null null)
    (`KismetSystemLibrary.Delay` 2.0)
    (bind _hudwidget (`self.HUDWidget`)
      (:`then`
        (`/Game/Blueprints/UI/HUD/WBP_HUD.HideSentence` _hudwidget)
        (`self.Attack`)
        (`KismetSystemLibrary.Delay` 0.5)
        (`self.EnableInput` null)
        (set `self.State` "NewEnumerator0"))
      (:`else`))
    (else
      (`GameplayStatics.PlaySound2D` "/Game/Audio/IncorrectInput.IncorrectInput" 1.0 1.0 0.0 null null)
      (`self.EndSpeech`)
      (set `self.State` "NewEnumerator0")
      (`KismetSystemLibrary.Delay` 2.0)
      (`self.BeginSpeech`))))

(fn `Attack`
  (for _array_element (`self.GetOverlappingActors` null)
    (bind _asbp_box (cast `/Game/Blueprints/Objects/BP_Box` _array_element))
    (bind _rendercomponent (`PaperSpriteActor.RenderComponent` _asbp_box))
    (`PrimitiveComponent.SetSimulatePhysics` _rendercomponent true)
    (`PrimitiveComponent.AddImpulse` _rendercomponent (100.0 0.0 400.0) "None" true)
    (`PrimitiveComponent.SetCollisionResponseToAllChannels` _rendercomponent "ECR_Ignore")
    (`PrimitiveComponent.SetCollisionResponseToAllChannels` (`/Game/Blueprints/Objects/BP_Box.CollisionBox` _asbp_box) "ECR_Ignore")
    (`PrimitiveComponent.SetCollisionResponseToAllChannels` (`/Game/Blueprints/Objects/BP_Box.Box` _asbp_box) "ECR_Ignore")
    (`self.PlayAttackEffects`)
    (`/Game/Blueprints/Objects/BP_Box.IsHit` _asbp_box)))

(fn `DestroyWidget`
  (`ActorComponent.K2_DestroyComponent` (`self.Widget`)))

(fn `GetCanMove`
  (returns (CanMove :type Boolean))
  (return (`self.CanMove`)))

(fn `GetHealth`
  (returns (Health :type Integer))
  (return (`self.Health`)))

(fn `GetState`
  (returns (State :type "/Game/Blueprints/Characters/E_PlayerStates Enum"))
  (return (`self.State`)))

(fn `LockMovement`
  (set `self.CanMove` false))

(fn `PlayAttackEffects`
  (`NiagaraFunctionLibrary.SpawnSystemAtLocation` "/Game/Effects/SlashEffect.SlashEffect" (+ (`self.K2_GetActorLocation`) (50.0 0.0 50.0)))
  (`GameplayStatics.PlaySound2D` "/Game/Audio/Sword_Swipe.Sword_Swipe" 1.0 1.0 0.0 null null))

(fn `TakeDamage`
  (bind _result (`/Engine/EditorBlueprintResources/StandardMacros.DecrementInt` (`self.Health`))
    (:`  `
      (bind _output_get (set `self.Health` (`KismetMathLibrary.Clamp` _result 0 3)))
      (if (<= _output_get 0)
        (bind _returnvalue (`|CreateWidget` "/Game/Blueprints/UI/HUD/WBP_LossMenu.WBP_LossMenu_C"))
        (`UserWidget.AddToViewport` _returnvalue 0)
        (`self.DisableInput` null)))))

(fn `UnlockMovement`
  (set `self.CanMove` true))

(fn `UpdateAnimation`
  (if (> (`KismetMathLibrary.VSize` (`self.GetVelocity`)) 0.0)
    ;[1 1 1] Running
    (`PaperFlipbookComponent.SetFlipbook` (`self.Sprite`) "/Game/PaperAssets/Characters/Knight/FlipBook/FB_Knight_Run.FB_Knight_Run")
    (else
      ;[1 1 1] Idle
      (`PaperFlipbookComponent.SetFlipbook` (`self.Sprite`) "/Game/PaperAssets/Characters/Knight/FlipBook/FB_Knight_Idle.FB_Knight_Idle"))))

(fn `UserConstructionScript`)